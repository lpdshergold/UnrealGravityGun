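; Door frame Blueprint whose door swings on a timeline and is unlocked by hitting pads in a set order.
; DoStepOnPad checks each hit against PadSequence, resetting progress on a wrong pad and triggering DoDoor when the sequence completes.
; DoDoor scales the timeline's sweep by MaxOpen to drive door yaw, then resets the timeline time when finished.
; BeginPlay also triggers the door after a short delay, independent of the lock.
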(event `self.ReceiveBeginPlay`
  (`KismetSystemLibrary.Delay` 3.0)
  (`self.DoDoor`))

(event `DoDoor`
  (bind (_direction _sweep) (`Timeline|DoorRotate` :`NewTime` 0.0 :!label _label)
    (:`Update`
      (`SceneComponent.K2_SetRelativeRotation` (`self.Door`) (`KismetMathLibrary.MakeRotator` 0.0 0.0 (* _sweep (`self.MaxOpen`))) false false))
    (:`Finished`
      (`self.DoNothing`)
      (goto _label :!via `SetNewTime`))))

(event `ResetLock`
  (set `self.currentStep` 0))

(event `DoStepOnPad`
  (params (HitPad :type "/Game/Blueprints/Pad_BP Object Reference"))
  (bind _padsequence (`self.PadSequence`))
  (if (== (`|GetArrayItem` _padsequence (`self.currentStep`)) HitPad)
    (bind _result (`/Engine/EditorBlueprintResources/StandardMacros.IncrementInt` (`self.currentStep`))
      (:`  `
        (if (== (`KismetArrayLibrary.Array_Length` _padsequence) _result)
          (`self.ResetLock`)
          (`self.DoDoor`))))
    (else
      (`self.ResetLock`))))

(fn `DoNothing`)

(fn `UserConstructionScript`)